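; AI controller that runs the BT_AI behavior tree on BeginPlay and tracks whether its AI perception senses the player.
; Perception updates for actors tagged Player write the isSeeingPlayer blackboard bool, true when sensed and false when lost.
; The first successful sighting also plays a scream at the perception owner's location, gated by a DoOnce that is never reset.
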(event `self.ReceiveBeginPlay`
  (`self.RunBehaviorTree` "/Game/AI/BT_AI.BT_AI"))

(event `self.AIPerception.OnTargetPerceptionUpdated`
  (params (Actor :type "Actor Object Reference") (Stimulus :type "AIStimulus Structure"))
  (if (`self.ActorHasTag` Actor "Player")
    (if (`.bSuccessfullySensed` (break `AIStimulus` Stimulus))
      (`BlackboardComponent.SetValueAsBool` (`AIBlueprintHelperLibrary.GetBlackboard` null) "isSeeingPlayer" true)
      (`/Engine/EditorBlueprintResources/StandardMacros.DoOnce` false
        (:`Completed`
          (`GameplayStatics.PlaySoundAtLocation` "/Game/Audio/MS_AIScream.MS_AIScream" (`self.K2_GetActorLocation` (`ActorComponent.GetOwner` (`self.AIPerception`))) (struct) 1.0 1.0 0.0 null null null null)))
      (else
        (`BlackboardComponent.SetValueAsBool` (`AIBlueprintHelperLibrary.GetBlackboard` null) "isSeeingPlayer" false)))))

(fn `UserConstructionScript`)